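; Constellation actor that shows a configurable mesh with a name label, both set up in the construction script.
; ToggleActive flips mesh and label visibility, then a timeline eases the "Emissive" parameter of two dynamic materials toward HighEmissive.
; FadeMaterials lerps from each material's current value rather than a stored start.
; OnFocus and LostFocus are empty; the CanHighlight-gated highlight fade logic is disconnected and never runs.
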(event `self.ReceiveBeginPlay`
  (bind _staticmesh (`self.StaticMesh`))
  (bind _staticmesh_2 (`self.StaticMesh`))
  ;[0 0 0] Begin Play - Create Dynamic Mats
  (bind _returnvalue (`PrimitiveComponent.CreateDynamicMaterialInstance` _staticmesh_2 0 (`PrimitiveComponent.GetMaterial` _staticmesh_2 0)))
  (set `self.Mat` _returnvalue)
  (bind _returnvalue_2 (`PrimitiveComponent.CreateDynamicMaterialInstance` _staticmesh 1 (`PrimitiveComponent.GetMaterial` _staticmesh 1)))
  (set `self.Mat2` _returnvalue_2))

(event `/Game/Blueprints/InteractableInterface.OnFocus`
  ;[0 0 0] Focus Events
)

(event `/Game/Blueprints/InteractableInterface.LostFocus`
  ;[0 0 0] Focus Events
)

(event `ToggleActive`
  (bind _highemissive (`self.HighEmissive`))
  (bind _mat (`self.Mat`))
  (bind _mat2 (`self.Mat2`))
  ;[0 0 0] Toggle All Active states of the Blueprint
  (`SceneComponent.ToggleVisibility` (`self.StaticMesh`) false)
  (`SceneComponent.ToggleVisibility` (`self.TextRender`) false)
  (bind (_direction _fade) (`Timeline|Timeline_1` :!via `PlayFromStart`)
    (:`Update`
      (`self.FadeMaterials` _mat _mat _highemissive _fade)
      (`self.FadeMaterials` _mat2 _mat2 _highemissive _fade))))

(fn `FadeMaterials`
  (params (self2 :type "MaterialInstanceDynamic Object Reference") (self3 :type "MaterialInstanceDynamic Object Reference") (EndValue :type "Float (double-precision)") (Alpha :type "Float (double-precision)"))
  (bind _returnvalue (`MaterialInstanceDynamic.K2_GetScalarParameterValue` self3 "Emissive"))
  (`MaterialInstanceDynamic.SetScalarParameterValue` self2 "Emissive" (`KismetMathLibrary.Lerp` _returnvalue EndValue Alpha)))

(fn `UserConstructionScript`
  (bind _textrender (`self.TextRender`))
  (`TextRenderComponent.K2_SetText` _textrender (`self.Name`))
  (`SceneComponent.K2_SetRelativeLocation` _textrender (`self.TextLocation`) false false)
  (`StaticMeshComponent.SetStaticMesh` (`self.StaticMesh`) (`self.Constellation`)))