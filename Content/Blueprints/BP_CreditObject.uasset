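; BP_CreditObject is a credit item with configurable text and a PStar effect that responds to a ControlHover event.
; The construction script sets the text and creates a dynamic material instance on the text component.
; The first hover deactivates PStar, toggles the text's visibility and sets Viewed, so later hovers do nothing.
; A timeline meant to animate a material parameter is unconnected and never runs.
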(event `/Game/Blueprints/InteractableInterface.ControlHover`
  (if (not (`self.bViewed`))
    (`ActorComponent.Deactivate` (`self.P_Star`))
    (`SceneComponent.ToggleVisibility` (`self.TextRender`) false)
    (set `self.bViewed` true)))

(fn `UserConstructionScript`
  (bind _textrender (`self.TextRender`))
  (`TextRenderComponent.K2_SetText` _textrender (`self.Text`))
  (bind _returnvalue (`PrimitiveComponent.CreateDynamicMaterialInstance` _textrender 0 null))
  (set `self.DynamicMat` _returnvalue))