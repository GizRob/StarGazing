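; VR player pawn for Google VR that focuses objects by gaze and hovers and clicks lamps with the motion controller.
; Each tick rotates the Arm to controller orientation and line-traces from Camera and Sphere, sending focus and hover messages when hit actors change.
; Thumbstick press or K sends the click message to the hovered lamp, through duplicated handlers.
; BeginPlay spawns a TraceVisualiser, but TraceEnd, which draws its line, is only called from unreachable nodes.
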(event `self.ReceiveBeginPlay`
  (bind _returnvalue (`|SpawnActorFromClass` "/Game/Blueprints/TraceVisualiser.TraceVisualiser_C" (`SceneComponent.K2_GetComponentToWorld` (`self.Sphere`)) "Undefined" "OverrideRootScale" null (1.0 1.0 1.0)))
  (set `self.Visualiser` _returnvalue))

(event `self.ReceiveTick`
  (params (DeltaSeconds :type "Float (single-precision)"))
  (`|ExecutionSequence`
    (:`then_0`
      (`self.GazeCheck`)
      (bind _returnvalue (`GoogleVRControllerFunctionLibrary.GetGoogleVRControllerOrientation`))
      (`SceneComponent.K2_SetWorldRotation` (`self.Arm`) _returnvalue false false))
    (:`then_1`
      (`self.ControllerCheck`))))

(event `GazeCheck`
  (bind _camera (`self.Camera`))
  (bind _focusedobject (`self.FocusedObject`))
  (bind _returnvalue (`SceneComponent.K2_GetComponentLocation` _camera))
  ;[1 1 1] Gaze Control
  (bind _outhit (`KismetSystemLibrary.LineTraceSingle` _returnvalue (+ _returnvalue (* (`SceneComponent.GetForwardVector` _camera) 100000.0)) "TraceTypeQuery1"))
  (bind (_bblockinghit _binitialoverlap _time _location _impactpoint _normal _impactnormal _physmat _hitactor) (`GameplayStatics.BreakHitResult` _outhit))
  (if (!= _hitactor _focusedobject)
    (message `/Game/Blueprints/InteractableInterface.LostFocus` _focusedobject)
    (message `/Game/Blueprints/InteractableInterface.OnFocus` _hitactor)
    (set `self.FocusedObject` _hitactor)))

(event `ControllerCheck`
  (bind _sphere (`self.Sphere`))
  (bind _focusedlamp (`self.FocusedLamp`))
  (bind _returnvalue (`SceneComponent.K2_GetComponentLocation` _sphere))
  (bind _outhit (`KismetSystemLibrary.LineTraceSingle` :`Start` _returnvalue :`End` (+ _returnvalue (* (`SceneComponent.GetForwardVector` _sphere) 1000.0)) :`TraceChannel` "TraceTypeQuery1" :`TraceColor` (struct :`G` 0.158242 :`B` 1.0 :`A` 1.0)))
  (bind (_bblockinghit _binitialoverlap _time _location _impactpoint _normal _impactnormal _physmat _hitactor) (`GameplayStatics.BreakHitResult` _outhit))
  (if (!= _hitactor _focusedlamp)
    (message `/Game/Blueprints/InteractableInterface.ControlLostHover` _focusedlamp)
    (message `/Game/Blueprints/InteractableInterface.ControlHover` _hitactor)
    (set `self.FocusedLamp` _hitactor)))

(event `Key|MotionController_Left_Thumbstick`
  (params (Key :type "Key Structure" :default "AnyKey"))
  (:`Pressed`
    (message `/Game/Blueprints/InteractableInterface.OnLampClicked` (`self.FocusedLamp`) :!label _label)))

(event `Key|K`
  (params (Key :type "Key Structure" :default "AnyKey"))
  (:`Pressed`
    (goto _label)))

(event `Key|MotionController_Left_Thumbstick`
  (params (Key :type "Key Structure" :default "AnyKey"))
  (:`Pressed`
    (message `/Game/Blueprints/InteractableInterface.OnLampClicked` (`self.FocusedLamp`) :!label _label_2)))

(event `Key|K`
  (params (Key :type "Key Structure" :default "AnyKey"))
  (:`Pressed`
    (goto _label_2)))

(fn `TraceEnd`
  (returns (OutHit :type "HitResult Structure"))
  (bind _sphere (`self.Sphere`))
  (bind _visualiser (`self.Visualiser`))
  (bind _returnvalue (`SceneComponent.K2_GetComponentLocation` _sphere))
  (bind _returnvalue_2 (+ _returnvalue (* (`SceneComponent.GetForwardVector` _sphere) 500.0)))
  (set `self.EndLocal` _returnvalue_2)
  (bind _outhit (`KismetSystemLibrary.LineTraceSingle` _returnvalue _returnvalue_2 "TraceTypeQuery1"))
  ;[1 1 1] Visualise trace
  (`/Engine/EditorBlueprintResources/StandardMacros.IsValid` _visualiser
    (:`Is Valid`
      (`/Game/Blueprints/TraceVisualiser.RenderLine` _visualiser _returnvalue (`self.EndLocal`) 100.0 5.0))
    (:`Is Not Valid`
      _))
  (return _outhit))

(fn `UserConstructionScript`)