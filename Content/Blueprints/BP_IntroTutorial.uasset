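; Intro tutorial actor that steps through text prompts with controller clicks, then hands off to the Zen_P level.
; BeginPlay creates dynamic materials and shows the first two prompts on a timer, after which clicks advance the text.
; Successive clicks reveal the mesh, then shrink it with a timeline while a FadeOut sequence plays before the level loads.
; Hover events tint the mesh and text materials yellow, restoring white afterward.
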(event `self.ReceiveBeginPlay`
  (bind _staticmesh (`self.StaticMesh`))
  (bind _returnvalue (`PrimitiveComponent.CreateDynamicMaterialInstance` _staticmesh 0 null))
  (set `self.mat1` _returnvalue)
  (bind _returnvalue_2 (`PrimitiveComponent.CreateDynamicMaterialInstance` _staticmesh 2 null))
  (set `self.mat2` _returnvalue_2)
  (bind _returnvalue_3 (`PrimitiveComponent.CreateDynamicMaterialInstance` (`self.TextRender`) 0 null))
  (set `self.TextMat` _returnvalue_3)
  (`self.UpdateCurrentText`)
  (`KismetSystemLibrary.Delay` 5.0)
  (`self.UpdateCurrentText`))

(event `/Game/Blueprints/InteractableInterface.ControlHover`
  (`MaterialInstanceDynamic.SetVectorParameterValue` (`self.mat1`) "Body" (struct :`R` 1.0 :`G` 1.0 :`A` 1.0))
  (`MaterialInstanceDynamic.SetVectorParameterValue` (`self.mat2`) "Body" (struct :`R` 1.0 :`G` 1.0 :`A` 1.0))
  (`MaterialInstanceDynamic.SetVectorParameterValue` (`self.TextMat`) "Body" (struct :`R` 1.0 :`G` 1.0 :`A` 1.0)))

(event `/Game/Blueprints/InteractableInterface.ControlLostHover`
  (`MaterialInstanceDynamic.SetVectorParameterValue` (`self.mat1`) "Body" (struct :`R` 1.0 :`G` 1.0 :`B` 1.0 :`A` 1.0))
  (`MaterialInstanceDynamic.SetVectorParameterValue` (`self.mat2`) "Body" (struct :`R` 1.0 :`G` 1.0 :`B` 1.0 :`A` 1.0))
  (`MaterialInstanceDynamic.SetVectorParameterValue` (`self.TextMat`) "Body" (struct :`R` 1.0 :`G` 1.0 :`B` 1.0 :`A` 1.0)))

(event `/Game/Blueprints/InteractableInterface.OnControllerClicked`
  (bind _staticmesh (`self.StaticMesh`))
  (if (>= (`self.CurrentText`) 2)
    (`self.UpdateCurrentText`)
    (if (== (`self.CurrentText`) 3)
      (`SceneComponent.SetHiddenInGame` (`self.StaticMesh`) false false)
      (elif (== (`self.CurrentText`) 4)
        (`|ExecutionSequence`
          (:`then_0`
            (bind (_direction _newtrack_0) (`Timeline|Timeline_0` :!via `PlayFromStart`)
              (:`Update`
                (`SceneComponent.SetWorldScale3D` _staticmesh (`KismetMathLibrary.VLerp` (`SceneComponent.K2_GetComponentScale` _staticmesh) (0.0 0.0 0.0) _newtrack_0)))))
          (:`then_1`
            (bind _returnvalue (`LevelSequencePlayer.CreateLevelSequencePlayer` "/Game/Cinematic/FadeOut.FadeOut"))
            (`LevelSequencePlayer.Play` _returnvalue)
            (`KismetSystemLibrary.Delay` 5.0)
            (`GameplayStatics.OpenLevel` "Zen_P")))))))

(event `UpdateCurrentText`
  ;[1 1 1] Update current Text
  (`TextRenderComponent.K2_SetText` (`self.TextRender`) (`KismetArrayLibrary.Array_Get` (`self.TextVals`) (`self.CurrentText`)))
  (set `self.CurrentText` (+ (`self.CurrentText`) 1)))

(fn `UserConstructionScript`)